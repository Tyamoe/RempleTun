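; Behavior tree task that gives a flying AI an approach or orbit position around the player, written to the OrbitPos Blackboard key.
; Out of range, it targets a standoff point on the line to the player and syncs the orbit angle to that heading.
; Within range, it steps the angle each execution in a randomly chosen direction, held until the pawn leaves range, to circle the player.
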(event Custom|UpdateAngle
  ;[1 1 1] Update Target Angle
  (if (Variables|Default|GetSet)
    _
    (else
      (Variables|Default|SetIncrease (Math|Random|RandomBool))
      (Variables|Default|SetSet true)))
  (if (Variables|Default|GetIncrease)
    (Variables|Default|SetAngle (Math|Float|Lerp (Variables|Default|GetAngle) (+ (Variables|Default|GetAngle) 1e+01) 0.5))
    (else
      (Variables|Default|SetAngle (Math|Float|Lerp (Variables|Default|GetAngle) (+ (Variables|Default|GetAngle) -1e+01) 0.5)))))

(event EventReceiveExecuteAI
  (params (OwnerController :type AI%20Controller%20Object%20Reference) (ControlledPawn :type Pawn%20Object%20Reference))
  (bind _returnvalue (Game|GetPlayerCharacter 0))
  (bind _returnvalue_2 (Transformation|GetActorLocation ControlledPawn))
  (bind _returnvalue_3 (Transformation|GetActorLocation _returnvalue))
  (bind _returnvalue_4 (Math|Vector|GetUnitDirection(Vector) _returnvalue_2 _returnvalue_3))
  (if (<= (Math|Vector|Distance(Vector) _returnvalue_2 _returnvalue_3) 4e+02)
    (CallFunction|UpdateAngle)
    (AI|BehaviorTree|SetBlackboardValueasVector (Variables|Default|GetOrbitPos) (+ (Transformation|GetActorLocation (Game|GetPlayerCharacter 0)) (* (Math|Vector|MakeVector (Math|Trig|Cos(Degrees) (Variables|Default|GetAngle)) (Math|Trig|Sin(Degrees) (Variables|Default|GetAngle)) (.Z (Math|Vector|BreakVector _returnvalue_4))) (Math|Float|MakeLiteralFloat -2.5e+02))))
    (AI|BehaviorTree|FinishExecute true)
    (else
      (Variables|Default|SetAngle (Math|Trig|RadiansToDegrees (Class|KismetMathLibrary|VectorHeadingAngle _returnvalue_4)))
      (bind _output_get (Variables|Default|SetOrbit (+ (* _returnvalue_4 (Math|Float|MakeLiteralFloat -2.5e+02)) _returnvalue_3)))
      (AI|BehaviorTree|SetBlackboardValueasVector (Variables|Default|GetOrbitPos) _output_get)
      (AI|BehaviorTree|FinishExecute true)
      (Variables|Default|SetSet false))))